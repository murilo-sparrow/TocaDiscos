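; BP_TocaDiscos is a record player actor with an animated dust cover, power, pause, mute and volume controls.
; Montages drive the cover and power switching; turning on requires an open cover, and closing it stops the music.
; After a short delay, power-on spawns a random track at the actor's location as a stored component that the controls adjust.
; Tick spins the vinyl while playing, and volume changes rotate a knob with a click sound.
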(event Custom|MuteMusic
  (bind _musiccomponent (Variables|Sound|GetMusicComponent)
    (:then
      (Audio|Components|Audio|SetVolumeMultiplier _musiccomponent 0.001 :!class /Script/Engine.AudioComponent)
      (Variables|Flags|SetIsMusicMute true))
    (:else)))

(event Custom|UnmuteMusic
  (bind _musiccomponent (Variables|Sound|GetMusicComponent)
    (:then
      (Audio|Components|Audio|SetVolumeMultiplier _musiccomponent (Variables|Sound|GetVolume) :!class /Script/Engine.AudioComponent)
      (Variables|Flags|SetIsMusicMute false))
    (:else)))

(event Custom|TogglePause
  (params (IsPaused :type Boolean))
  (bind _output_get (Variables|Flags|SetIs%20Paused (!= true IsPaused)))
  (bind _musiccomponent (Variables|Sound|GetMusicComponent)
    (:then
      (Class|AudioComponent|SetPaused _musiccomponent _output_get))
    (:else)))

(event Custom|TurnOff
  (Animation|Montage|PlayMontage (Variables|Components|GetTocaDiscos) "/Game/Art/Animations/AM_VinilPlayer_TurningOff.AM_VinilPlayer_TurningOff" 3.0
    (:then
      (Variables|Flags|SetIsTocaDiscosOn false)
      (CallFunction|StopMusic))))

(event Custom|ChangeVolume
  (params (InputValue :type Float%20%28double-precision%29))
  (bind _output_get (Variables|Sound|SetVolume (Math|Float|Clamp(Float) (+ (Variables|Sound|GetVolume) (* InputValue 0.05)) 0.001 4.0)))
  (if (!= _output_get (Variables|Sound|GetLastVolume))
    (Variables|Sound|SetLastVolume (Variables|Sound|GetVolume))
    (bind _musiccomponent (Variables|Sound|GetMusicComponent)
      (:then
        (Audio|Components|Audio|SetVolumeMultiplier _musiccomponent (Variables|Sound|GetVolume) :!class /Script/Engine.AudioComponent)
        (Transformation|AddLocalRotation (Variables|Components|GetVolumeSpin) (Math|Rotator|MakeRotator (* InputValue -2.0) 0.0 0.0) false false)
        (Audio|PlaySound2D "/Engine/VREditor/Sounds/UI/Click_on_Button.Click_on_Button" 0.3 1.0 0.0 0 0))
      (:else))))

(event Custom|ToggleMute
  (if (Variables|Flags|GetIsMusicMute)
    (CallFunction|UnmuteMusic)
    (else
      (CallFunction|MuteMusic))))

(event Custom|ToggleOnOff
  (if (Variables|Flags|GetIsTocaDiscosOn)
    (CallFunction|TurnOff)
    (else
      (CallFunction|Turnon))))

(event Custom|TurnOn
  (if (not (Variables|Flags|GetIsCoverClose))
    (Animation|Montage|PlayMontage (Variables|Components|GetTocaDiscos) "/Game/Art/Animations/AM_VinilPlayer_TurningOn.AM_VinilPlayer_TurningOn" 3.0
      (:then
        (Utilities|FlowControl|Delay 1.25)
        (Variables|Flags|SetIsTocaDiscosOn true)
        (CallFunction|StartMusic)))))

(event Custom|DustCoverOpening
  (Animation|Montage|PlayMontage (Variables|Components|GetTocaDiscos) "/Game/Art/Animations/AM_RPDustCover_Opening.AM_RPDustCover_Opening" 3.0
    (:then
      (Variables|Flags|SetIsCoverClose false))))

(event Custom|DustCoverClosing
  (Animation|Montage|PlayMontage (Variables|Components|GetTocaDiscos) "/Game/Art/Animations/AM_RPDustCover_Closing.AM_RPDustCover_Closing" 3.0
    (:then
      (Variables|Flags|SetIsCoverClose true)
      (Variables|Flags|SetIsTocaDiscosOn false)
      (CallFunction|StopMusic))))

(event Custom|ToggleCover
  (if (Variables|Flags|GetIsCoverClose)
    (CallFunction|DustCoverOpening)
    (else
      (CallFunction|DustCoverClosing))))

(event EventBeginPlay)

(event EventTick
  (params (DeltaSeconds :type Float%20%28single-precision%29))
  (if (not (Variables|Flags|GetIs%20Paused))
    (if (Variables|Flags|GetIsTocaDiscosOn)
      (Transformation|AddLocalRotation (Variables|Default|GetVinil) (Math|Rotator|MakeRotator 0.0 0.0 0.8) false false))))

(fn ConstructionScript)

(fn StartMusic
  (bind _returnvalue (Audio|SpawnSoundatLocation (.OutItem (Utilities|Array|Random (Variables|Sound|GetMusics))) (Transformation|GetActorLocation) "0, 0, 0" (Variables|Sound|GetVolume) 1.0 0.0 0 0))
  (Variables|Sound|SetMusicComponent _returnvalue))

(fn StopMusic
  (bind _musiccomponent (Variables|Sound|GetMusicComponent)
    (:then
      (Audio|Components|Audio|Stop _musiccomponent))
    (:else)))