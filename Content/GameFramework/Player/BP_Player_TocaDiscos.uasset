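; First-person player Blueprint for looking around, zooming and operating a record player (BP_TocaDiscos).
; A per-tick camera line trace caches the last hit actor and component, never clearing them on a miss.
; Enhanced Input forwards cover, mute, power and volume actions to that actor, with volume requiring a tagged component.
; Pause needs a cached record player, swaps UI widgets, blocks other input and lets Escape quit.
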(event Input|EnhancedActionEvents|EnhancedInputActionIA_CameraZoom
  (params (ActionValue :type Boolean) (ElapsedSeconds :type Float%20%28double-precision%29) (TriggeredSeconds :type Float%20%28double-precision%29) (InputAction :type Input%20Action%20Object%20Reference :default "/Game/Input/IA_CameraZoom.IA_CameraZoom"))
  (bind _camera (Variables|Default|GetCamera))
  (bind _ispauseon (Variables|Default|GetIsPauseOn))
  (:Started
    (if (not _ispauseon)
      (Camera|SetFieldOfView _camera 5e+01)))
  (:Completed
    (if (not _ispauseon)
      (Camera|SetFieldOfView _camera 9e+01))))

(event Input|EnhancedActionEvents|EnhancedInputActionIA_ChangeVolume
  (params (ActionValue :type Float%20%28double-precision%29) (ElapsedSeconds :type Float%20%28double-precision%29) (TriggeredSeconds :type Float%20%28double-precision%29) (InputAction :type Input%20Action%20Object%20Reference :default "/Game/Input/IA_ChangeVolume.IA_ChangeVolume"))
  (if (not (Variables|Default|GetIsPauseOn))
    (bind _hittocadiscoscomponent (Variables|Default|GetHitTocaDiscosComponent)
      (:then
        (if (Components|ComponentHasTag _hittocadiscoscomponent "VolumeBoxColision")
          (bind _asbp_toca_discos (Utilities|Casting|CastToBP_TocaDiscos (Variables|Default|GetHitTocaDiscos)))
          (Default|ChangeVolume _asbp_toca_discos ActionValue)))
      (:else))))

(event Input|EnhancedActionEvents|EnhancedInputActionIA_CameraMovement
  (params (ActionValue :type Vector%202D%20Structure) (ElapsedSeconds :type Float%20%28double-precision%29) (TriggeredSeconds :type Float%20%28double-precision%29) (InputAction :type Input%20Action%20Object%20Reference :default "/Game/Input/IA_CameraMovement.IA_CameraMovement"))
  (if (not (Variables|Default|GetIsPauseOn))
    (Pawn|Input|AddControllerYawInput (.x ActionValue))
    (Pawn|Input|AddControllerPitchInput (* (.y ActionValue) -1.0))))

(event Input|EnhancedActionEvents|EnhancedInputActionIA_PauseMenu
  (params (ActionValue :type Boolean) (ElapsedSeconds :type Float%20%28double-precision%29) (TriggeredSeconds :type Float%20%28double-precision%29) (InputAction :type Input%20Action%20Object%20Reference :default "/Game/Input/IA_PauseMenu.IA_PauseMenu"))
  (:Started
    (bind _asbp_toca_discos (Utilities|Casting|CastToBP_TocaDiscos (Variables|Default|GetHitTocaDiscos)))
    (Default|TogglePause _asbp_toca_discos (Variables|Default|GetIsPauseOn))
    (if (Variables|Default|GetIsPauseOn)
      (Viewport|RemoveAllWidgets)
      (bind _returnvalue (UserInterface|CreateWidget "/Game/Blueprints/Widgets/WBP_TocaDiscos_MainUI.WBP_TocaDiscos_MainUI_C"))
      (UserInterface|Viewport|AddtoViewport _returnvalue 0)
      (Variables|Default|SetIsPauseOn false)
      (else
        (bind _returnvalue_2 (UserInterface|CreateWidget "/Game/Blueprints/Widgets/WBP_PauseMenu.WBP_PauseMenu_C"))
        (UserInterface|Viewport|AddtoViewport _returnvalue_2 0)
        (Variables|Default|SetIsPauseOn true)))))

(event Input|EnhancedActionEvents|EnhancedInputActionIA_Mute
  (params (ActionValue :type Boolean) (ElapsedSeconds :type Float%20%28double-precision%29) (TriggeredSeconds :type Float%20%28double-precision%29) (InputAction :type Input%20Action%20Object%20Reference :default "/Game/Input/IA_Mute.IA_Mute"))
  (:Completed
    (if (not (Variables|Default|GetIsPauseOn))
      (bind _asbp_toca_discos (Utilities|Casting|CastToBP_TocaDiscos (Variables|Default|GetHitTocaDiscos)))
      (Default|ToggleMute _asbp_toca_discos))))

(event Input|EnhancedActionEvents|EnhancedInputActionIA_Cover
  (params (ActionValue :type Boolean) (ElapsedSeconds :type Float%20%28double-precision%29) (TriggeredSeconds :type Float%20%28double-precision%29) (InputAction :type Input%20Action%20Object%20Reference :default "/Game/Input/IA_Cover.IA_Cover"))
  (:Completed
    (if (not (Variables|Default|GetIsPauseOn))
      (bind _asbp_toca_discos (Utilities|Casting|CastToBP_TocaDiscos (Variables|Default|GetHitTocaDiscos)))
      (Default|ToggleCover _asbp_toca_discos))))

(event Input|EnhancedActionEvents|EnhancedInputActionIA_TurnOnOff
  (params (ActionValue :type Boolean) (ElapsedSeconds :type Float%20%28double-precision%29) (TriggeredSeconds :type Float%20%28double-precision%29) (InputAction :type Input%20Action%20Object%20Reference :default "/Game/Input/IA_TurnOnOff.IA_TurnOnOff"))
  (:Completed
    (if (not (Variables|Default|GetIsPauseOn))
      (bind _asbp_toca_discos (Utilities|Casting|CastToBP_TocaDiscos (Variables|Default|GetHitTocaDiscos)))
      (Default|ToggleonOff _asbp_toca_discos))))

(event EventBeginPlay
  (Input|AddMappingContext (PlayerController|LocalPlayerSubsystems|GetEnhancedInputLocalPlayerSubsystem (Game|GetPlayerController 0)) "/Game/Input/IMC_TocaDiscos.IMC_TocaDiscos" 0 "(bIgnoreAllPressedKeysUntilRelease=True,bForceImmediately=False,bNotifyUserSettings=False)")
  (bind _returnvalue (UserInterface|CreateWidget "/Game/Blueprints/Widgets/WBP_TocaDiscos_MainUI.WBP_TocaDiscos_MainUI_C"))
  (UserInterface|Viewport|AddtoViewport _returnvalue 0))

(event EventTick
  (params (DeltaSeconds :type Float%20%28single-precision%29))
  (CallFunction|ExecuteLineTrace))

(event Input|KeyboardEvents|Escape
  (params (Key :type Key%20Structure :default "None"))
  (:Released
    (if (Variables|Default|GetIsPauseOn)
      (Game|QuitGame 0 "Quit" false))))

(fn ConstructionScript)

(fn ExecuteLineTrace
  (bind _camera (Variables|Default|GetCamera))
  (bind _returnvalue (Transformation|GetWorldLocation _camera))
  (bind (_outhit _returnvalue_2) (Collision|LineTraceByChannel _returnvalue (+ _returnvalue (* (Math|Vector|GetForwardVector _camera) 2e+02)) "TraceTypeQuery1" false 0 "None"))
  (if _returnvalue_2
    (Variables|Default|SetHitTocaDiscos (.hitactor _outhit))
    (Variables|Default|SetHitTocaDiscosComponent (.hitcomponent _outhit))))